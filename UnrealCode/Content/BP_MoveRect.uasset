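; BP_MoveRect is an actor that moves its StaticMesh around a rectangular path in the local X-Z plane.
; Each Tick, a switch on the MoveType enum steps the stored X or Z position by a fixed amount and applies it as the relative location.
; Reaching each edge limit advances the state through Right, Up, Left and Down in a loop.
; Movement is per frame without delta time, so speed depends on frame rate.
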(event `self.ReceiveBeginPlay`)

(event `self.ReceiveTick`
  (params (DeltaSeconds :type "Float (single-precision)"))
  (switch `/Game/EN_MoveType` (`self.MoveType`)
    (:`NewEnumerator0`
      ;[1 1 1] 오른쪽으로 이동
      (bind _output_get (set `self.X위치` (+ (`self.X위치`) 1.0)))
      (`SceneComponent.K2_SetRelativeLocation` (`self.StaticMesh`) (`KismetMathLibrary.MakeVector` _output_get 0.0 (`self.Z`)) false false)
      (if (>= (`self.X위치`) 200.0)
        (set `self.MoveType` "NewEnumerator1")))
    (:`NewEnumerator1`
      ;[1 1 1] 위로 이동
      (bind _output_get_2 (set `self.Z` (+ (`self.Z`) 1.0)))
      (`SceneComponent.K2_SetRelativeLocation` (`self.StaticMesh`) (`KismetMathLibrary.MakeVector` (`self.X위치`) 0.0 _output_get_2) false false)
      (if (>= (`self.Z`) 400.0)
        (set `self.MoveType` "NewEnumerator2")))
    (:`NewEnumerator2`
      ;[1 1 1] 왼쪽으로 이동
      (bind _output_get_3 (set `self.X위치` (+ (`self.X위치`) -1.0)))
      (`SceneComponent.K2_SetRelativeLocation` (`self.StaticMesh`) (`KismetMathLibrary.MakeVector` _output_get_3 0.0 (`self.Z`)) false false)
      (if (<= (`self.X위치`) -200.0)
        (set `self.MoveType` "NewEnumerator3")))
    (:`NewEnumerator3`
      ;[1 1 1] 아래로 이동
      (bind _output_get_4 (set `self.Z` (+ (`self.Z`) -1.0)))
      (`SceneComponent.K2_SetRelativeLocation` (`self.StaticMesh`) (`KismetMathLibrary.MakeVector` (`self.X위치`) 0.0 _output_get_4) false false)
      (if (<= (`self.Z`) 0.0)
        (set `self.MoveType` "NewEnumerator0")))))

(fn `UserConstructionScript`)